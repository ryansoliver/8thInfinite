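; BP_RomulusGameMode is a game mode that respawns the player and enemies through custom events.
; Both events wait a short delay, then spawn a new actor of the passed-in actor's class at a shared RespawnTransform.
; RespawnPlayer has player controller 0 possess the new actor.
; RespawnEnemy uses a longer delay and skips possession, so the player does not take over respawned enemies.
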(event `Respawn Player`
  (params (Player :type "Character Object Reference"))
  ;[1 1 1] Respawn a player at Respawn Transform after a delay when destroyed
  (`KismetSystemLibrary.Delay` 0.2)
  (bind _returnvalue (`|SpawnActorFromClass` (`GameplayStatics.GetObjectClass` Player) (`self.Respawn Transform`) "Undefined" "MultiplyWithRoot" null null))
  (`Controller.Possess` (`GameplayStatics.GetPlayerController` 0) _returnvalue))

(event `RespawnEnemy`
  (params (Enemy :type "Character Object Reference"))
  ; Alternate Reapawn for enemy, so character doesn't get possessed after killing enemy
  (`KismetSystemLibrary.Delay` 2.0)
  (`|SpawnActorFromClass` (`GameplayStatics.GetObjectClass` Enemy) (`self.Respawn Transform`) "Undefined" "MultiplyWithRoot" null null))

(fn `UserConstructionScript`)