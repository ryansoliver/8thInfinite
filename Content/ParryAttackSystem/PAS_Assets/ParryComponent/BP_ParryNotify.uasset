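; BP_ParryNotify is an animation notify, named "Parry Attack", that marks an attack as part of the parry system.
; It passes its parryable, counter-attack and reaction montage settings to the owner's AC_ParryAttack component, if one exists.
; When the indicator option is on, it also triggers attack anticipation on that component and attaches a marker particle effect to the mesh's root as a telegraph.
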(fn `GetNotifyName`
  (returns (ReturnValue :type String))
  (return "Parry Attack"))

(fn `Received_Notify`
  (params (MeshComp :type "SkeletalMeshComponent Object Reference") (Animation :type "AnimSequenceBase Object Reference") (EventReference :type "AnimNotifyEventReference Structure (by ref)"))
  (returns (ReturnValue :type Boolean))
  (bind (_attackindicator_markervfx _attackindicator_markerlocationoffsetrootbone _attackindicator_markerscale _attackindicator_attackanticipateduration) (break `/Game/ParryAttackSystem/PAS_Assets/ParryComponent/F_AttackMarker` (`self.AttackIndicator`)))
  (bind (_reaction_montages_reactionmontageattacker _reaction_montages_reactionmontagedefender) (break `/Game/ParryAttackSystem/PAS_Assets/ParryComponent/F_ReactionsAnims` (`self.Reaction Montages`)))
  (bind (_attackindicator_markervfx_2 _attackindicator_markerlocationoffsetrootbone_2 _attackindicator_markerscale_2) (break `/Game/ParryAttackSystem/PAS_Assets/ParryComponent/F_AttackMarker` (`self.AttackIndicator`)))
  (bind _returnvalue (`Actor.GetComponentByClass` (`ActorComponent.GetOwner` MeshComp) "/Game/ParryAttackSystem/PAS_Assets/ParryComponent/AC_ParryAttack.AC_ParryAttack_C"))
  (`/Engine/EditorBlueprintResources/StandardMacros.IsValid` _returnvalue
    (:`Is Valid`
      (message `/Game/ParryAttackSystem/PAS_Assets/ParryComponent/BI_ParryInterface.SetParryAttack` _returnvalue (`self.Can be Parried?`) (`self.Is Counter Attack?`) (`self.Counter Attack Montages`) (`self.Use Reaction Anim?`) _reaction_montages_reactionmontageattacker _reaction_montages_reactionmontagedefender)
      (if (`self.UseParryAattackIndicator`)
        (`/Game/ParryAttackSystem/PAS_Assets/ParryComponent/AC_ParryAttack.Attack Anticipation` _returnvalue _attackindicator_attackanticipateduration)
        (`GameplayStatics.SpawnEmitterAttached` _attackindicator_markervfx_2 MeshComp "Root" _attackindicator_markerlocationoffsetrootbone_2 (struct) _attackindicator_markerscale_2)
        (return false)
        (else
          (return false))))))