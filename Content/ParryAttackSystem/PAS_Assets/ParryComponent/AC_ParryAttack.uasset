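; Actor component that gives characters timed parries, counter-attacks and front or back finishers.
; A parry inside the input window triggers a counter or reaction montage, using settings BP_ParryNotify supplies along with anticipation slow-mo.
; Finishers capsule-trace for a victim, check facing and randomly pick entries from DT_Finishers by the victim's CharacterName.
; Paired montages align both actors, temporarily disable collision, then apply damage or optional instant-kill ragdoll.
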(event `/Game/ParryAttackSystem/PAS_Assets/ParryComponent/BI_ParryInterface.SetParryAttack`
  (params (`CanBeParried?` :type Boolean) (`IsCounterAttack?` :type Boolean) (CounterAttackMontages :type "/Game/ParryAttackSystem/PAS_Assets/ParryComponent/F_FinisherStruct Structure") (`UseReactionAnim?` :type Boolean) (`ReactionMontage (Attacker)` :type "AnimMontage Object Reference") (`ReactionMontage (Defender)` :type "AnimMontage Object Reference"))
  ;[0 0 0] Set all parry variables - called from BP_ParryNotify
  (set `self.Can be Parried?` `CanBeParried?`)
  (set `self.Is Counter Attack?` `IsCounterAttack?`)
  (set `self.Counter Attack Montages` CounterAttackMontages)
  (set `self.Use Reaction Anim?` `UseReactionAnim?`)
  (set `self.Reaction Montage (Attacker)` `ReactionMontage (Attacker)`)
  (set `self.Reaction Montage (Defender)` `ReactionMontage (Defender)`))

(event `Uncrouch Event`
  (params (Target :type "Actor Object Reference"))
  (bind _returnvalue (`Actor.GetComponentByClass` Target "AC_ParryAttack_C"))
  ;[0 0 0] Uncrouch Dispatcher Event - Used on Finisher Event
  (`/Engine/EditorBlueprintResources/StandardMacros.IsValid` _returnvalue
    (:`Is Valid`
      (`self.UncrouchEvent` _returnvalue))))

(event `Attack Anticipation`
  (params (AnticipateDuration :type "Float (double-precision)"))
  (bind _returnvalue (`self.GetOwner`))
  ;[0 0 0] Attack Anticipation slowmo is called from BP_ParryNotify
  (set `Actor.CustomTimeDilation` 0.2 _returnvalue)
  (`KismetSystemLibrary.Delay` AnticipateDuration)
  (set `Actor.CustomTimeDilation` 1.0 _returnvalue))

(event `Finisher Event`
  (bind _front_finishers (`self.Front Finishers`))
  (bind _back_finishers (`self.Back Finishers`))
  (bind _returnvalue (`Actor.GetComponentByClass` (`self.VictimActor`) "/Script/Engine.CharacterMovementComponent"))
  (bind _returnvalue_2 (`Actor.GetComponentByClass` (`self.VictimActor`) "AC_ParryAttack_C"))
  (bind _returnvalue_3 (`Actor.GetComponentByClass` (`self.VictimActor`) "AC_ParryAttack_C"))
  (bind _returnvalue_4 (`SkeletalMeshComponent.GetAnimInstance` (`Actor.GetComponentByClass` (`self.GetOwner`) "/Script/Engine.SkeletalMeshComponent")))
  (bind _returnvalue_5 (`SkeletalMeshComponent.GetAnimInstance` (`Actor.GetComponentByClass` (`self.VictimActor`) "/Script/Engine.SkeletalMeshComponent")))
  (bind (_output_victimmontage _output_attackermontage _output_excdistance _output_instakill_ _output_useragdoll_ _output_timetoragdoll _output_damagetodo) (break `/Game/ParryAttackSystem/PAS_Assets/ParryComponent/F_FinisherStruct` (`|GetArrayItem` _back_finishers (`KismetMathLibrary.RandomIntegerInRange` 0 (- (`KismetArrayLibrary.Array_Length` _back_finishers) 1)))))
  (bind (_output_victimmontage_2 _output_attackermontage_2 _output_excdistance_2 _output_instakill__2 _output_useragdoll__2 _output_timetoragdoll_2 _output_damagetodo_2) (break `/Game/ParryAttackSystem/PAS_Assets/ParryComponent/F_FinisherStruct` (`|GetArrayItem` _front_finishers (`KismetMathLibrary.RandomIntegerInRange` 0 (- (`KismetArrayLibrary.Array_Length` _front_finishers) 1)))))
  ;[0 0 0] Finisher Event includes setting characters transforms and playing montages
  (`|ExecutionSequence`
    (:`then_0`
      (`self.SetVictim`))
    (:`then_1`
      (`self.CanExcFinisher?`
        (:`true`
          (if (`NavMovementComponent.IsCrouching` (`Actor.GetComponentByClass` (`self.GetOwner`) "/Script/Engine.CharacterMovementComponent"))
            (`self.Uncrouch Event` (`self.GetOwner`)))
          (`/Engine/EditorBlueprintResources/StandardMacros.IsValid` _returnvalue
            (:`Is Valid`
              (if (`NavMovementComponent.IsCrouching` _returnvalue)
                (`self.Uncrouch Event` (`self.VictimActor`))
                (`KismetSystemLibrary.Delay` 0.2)))
            (:`Is Not Valid`
              _))
          (if (`self.FinishFromBehind?`)
            (set `self.VictimMontage` _output_victimmontage)
            (set `self.AttackMontage` _output_attackermontage)
            (set `self.FinisherDistance` _output_excdistance)
            (set `self.IsInstaKill` _output_instakill_)
            (set `self.Use Ragdoll?` _output_useragdoll_)
            (set `self.Time to Ragdoll` _output_timetoragdoll)
            (set `self.DamageToDo` _output_damagetodo)
            (else
              (set `self.VictimMontage` _output_victimmontage_2)
              (set `self.AttackMontage` _output_attackermontage_2)
              (set `self.FinisherDistance` _output_excdistance_2)
              (set `self.IsInstaKill` _output_instakill__2)
              (set `self.Use Ragdoll?` _output_useragdoll__2)
              (set `self.Time to Ragdoll` _output_timetoragdoll_2)
              (set `self.DamageToDo` _output_damagetodo_2)))
          (`self.CalculateFinisherTransform`)
          (`|ExecutionSequence`
            (:`then_0`
              (`self.SetMovement/Collision` (`self.GetOwner`) "MOVE_Flying")
              (`/Engine/EditorBlueprintResources/StandardMacros.IsValid` _returnvalue_4
                (:`Is Valid`
                  (bind _returnvalue_6 (`AnimInstance.Montage_Play` _returnvalue_4 (`self.AttackMontage`) 1.0 "Duration" 0.0 true))
                  (set `self.IsParryMontagePlaying` true)
                  (`KismetSystemLibrary.Delay` (* _returnvalue_6 0.8))
                  (set `self.IsParryMontagePlaying` false)
                  (`self.SetMovement/Collision` (`self.GetOwner`) "MOVE_Walking" "QueryAndPhysics"))))
            (:`then_1`
              (`self.SetMovement/Collision` (`self.VictimActor`) "MOVE_Flying")
              (`/Engine/EditorBlueprintResources/StandardMacros.IsValid` _returnvalue_5
                (:`Is Valid`
                  (bind _returnvalue_7 (`AnimInstance.Montage_Play` _returnvalue_5 (`self.VictimMontage`) 1.0 "MontageLength" 0.0 true))
                  (if (`self.IsInstaKill`)
                    (set `/Game/ParryAttackSystem/PAS_Assets/ParryComponent/AC_ParryAttack.IsParryMontagePlaying` true _returnvalue_3)
                    (if (`self.Use Ragdoll?`)
                      (`KismetSystemLibrary.Delay` (`self.Time to Ragdoll`))
                      (set `/Game/ParryAttackSystem/PAS_Assets/ParryComponent/AC_ParryAttack.IsAlive` false _returnvalue_3)
                      (`self.Ragdoll Event` (`self.VictimActor`)))
                    (else
                      (set `/Game/ParryAttackSystem/PAS_Assets/ParryComponent/AC_ParryAttack.IsParryMontagePlaying` true _returnvalue_2)
                      (`KismetSystemLibrary.Delay` (* _returnvalue_7 0.8))
                      (set `/Game/ParryAttackSystem/PAS_Assets/ParryComponent/AC_ParryAttack.IsParryMontagePlaying` false _returnvalue_2)
                      (`self.SetMovement/Collision` (`self.VictimActor`) "MOVE_Walking" "QueryAndPhysics")
                      (`GameplayStatics.ApplyDamage` (`self.VictimActor`) (`self.DamageToDo`) null (`self.GetOwner`)))))))))))))

(event `TryParryAttack`
  (params (Pressed :type Boolean))
  ;[0 0 0] Parry Window Event
  (if Pressed
    (set `self.IsTryParry?` true)
    (`KismetSystemLibrary.RetriggerableDelay` (`self.ParryWindow`))
    (set `self.IsTryParry?` false)
    (else
      (set `self.IsTryParry?` false))))

(event `Ragdoll Event`
  (params (TargetActor :type "Actor Object Reference"))
  (bind _returnvalue (`Actor.GetComponentByClass` TargetActor "/Script/Engine.SkeletalMeshComponent"))
  (bind _returnvalue_2 (`Actor.GetComponentByClass` TargetActor "/Script/Engine.CapsuleComponent"))
  ;[0.1385 0 0.02935] Ragdoll Event
  (`PrimitiveComponent.SetCollisionEnabled` _returnvalue_2 "QueryAndPhysics")
  (`PrimitiveComponent.SetCollisionResponseToAllChannels` _returnvalue_2 "ECR_Ignore")
  (`PrimitiveComponent.SetCollisionResponseToChannel` _returnvalue_2 "ECC_WorldStatic" "ECR_Block")
  (`PrimitiveComponent.SetCollisionProfileName` _returnvalue "Ragdoll" true)
  (`PrimitiveComponent.SetSimulatePhysics` _returnvalue true)
  (`AnimInstance.Montage_Stop` (`SkeletalMeshComponent.GetAnimInstance` _returnvalue) 0.0 null))

(event `Parry Event`
  (bind _attackerpa (`self.AttackerPA`))
  (bind _reaction_montage__attacker_ (`/Game/ParryAttackSystem/PAS_Assets/ParryComponent/AC_ParryAttack.Reaction Montage (Attacker)` (`self.AttackerPA`)))
  (bind (_victimmontage _attackermontage _excdistance _instakill_ _useragdoll_ _timetoragdoll _damagetodo) (break `/Game/ParryAttackSystem/PAS_Assets/ParryComponent/F_FinisherStruct` (`/Game/ParryAttackSystem/PAS_Assets/ParryComponent/AC_ParryAttack.Counter Attack Montages` (`self.AttackerPA`))))
  (bind _returnvalue (`SkeletalMeshComponent.GetAnimInstance` (`Actor.GetComponentByClass` (`self.Attacker`) "/Script/Engine.SkeletalMeshComponent")))
  (bind _returnvalue_2 (`SkeletalMeshComponent.GetAnimInstance` (`Actor.GetComponentByClass` (`self.GetOwner`) "/Script/Engine.SkeletalMeshComponent")))
  ;[0 0 0] Parry Event is called when parry is successful
  (if (`/Game/ParryAttackSystem/PAS_Assets/ParryComponent/AC_ParryAttack.Is Counter Attack?` (`self.AttackerPA`))
    (set `self.VictimMontage` _victimmontage)
    (set `self.AttackMontage` _attackermontage)
    (set `self.FinisherDistance` _excdistance)
    (set `self.IsInstaKill` _instakill_)
    (set `self.Use Ragdoll?` _useragdoll_)
    (set `self.DamageToDo` _damagetodo)
    (set `self.Time to Ragdoll` _timetoragdoll)
    (`self.CalculateCounterTransform`)
    (`|ExecutionSequence`
      (:`then_0`
        (`self.SetMovement/Collision` (`self.GetOwner`) "MOVE_Flying")
        (`/Engine/EditorBlueprintResources/StandardMacros.IsValid` _returnvalue_2
          (:`Is Valid`
            (bind _returnvalue_3 (`AnimInstance.Montage_Play` _returnvalue_2 (`self.AttackMontage`) 1.0 "MontageLength" 0.0 true))
            (set `self.IsParryMontagePlaying` true)
            (`KismetSystemLibrary.Delay` (* _returnvalue_3 0.8))
            (set `self.IsParryMontagePlaying` false)
            (`self.SetMovement/Collision` (`self.GetOwner`) "MOVE_Walking" "QueryAndPhysics"))))
      (:`then_1`
        (`self.SetMovement/Collision` (`self.Attacker`) "MOVE_Flying")
        (`/Engine/EditorBlueprintResources/StandardMacros.IsValid` _returnvalue
          (:`Is Valid`
            (bind _returnvalue_4 (`AnimInstance.Montage_Play` _returnvalue (`self.VictimMontage`) 1.0 "MontageLength" 0.0 true))
            (if (`self.IsInstaKill`)
              (set `/Game/ParryAttackSystem/PAS_Assets/ParryComponent/AC_ParryAttack.IsParryMontagePlaying` true (`self.AttackerPA`))
              (if (`self.Use Ragdoll?`)
                (`KismetSystemLibrary.Delay` (`self.Time to Ragdoll`))
                (set `/Game/ParryAttackSystem/PAS_Assets/ParryComponent/AC_ParryAttack.IsAlive` false (`self.AttackerPA`))
                (`self.Ragdoll Event` (`self.Attacker`)))
              (else
                (set `/Game/ParryAttackSystem/PAS_Assets/ParryComponent/AC_ParryAttack.IsParryMontagePlaying` true _attackerpa)
                (`KismetSystemLibrary.Delay` (* _returnvalue_4 0.8))
                (set `/Game/ParryAttackSystem/PAS_Assets/ParryComponent/AC_ParryAttack.IsParryMontagePlaying` false _attackerpa)
                (`self.SetMovement/Collision` (`self.Attacker`) "MOVE_Walking" "QueryAndPhysics")
                (`GameplayStatics.ApplyDamage` (`self.Attacker`) (`self.DamageToDo`) null (`self.GetOwner`))))))))
    (elif (`/Game/ParryAttackSystem/PAS_Assets/ParryComponent/AC_ParryAttack.Use Reaction Anim?` (`self.AttackerPA`))
      (`|ExecutionSequence`
        (:`then_0`
          (`/Engine/EditorBlueprintResources/StandardMacros.IsValid` _reaction_montage__attacker_
            (:`Is Valid`
              (bind _returnvalue_5 (`AnimInstance.Montage_Play` (`SkeletalMeshComponent.GetAnimInstance` (`Actor.GetComponentByClass` (`self.Attacker`) "/Script/Engine.SkeletalMeshComponent")) _reaction_montage__attacker_ 1.0 "MontageLength" 0.0 true))
              (set `/Game/ParryAttackSystem/PAS_Assets/ParryComponent/AC_ParryAttack.IsParryMontagePlaying` true (`self.AttackerPA`))
              (`KismetSystemLibrary.Delay` (* _returnvalue_5 0.8))
              (set `/Game/ParryAttackSystem/PAS_Assets/ParryComponent/AC_ParryAttack.IsParryMontagePlaying` false (`self.AttackerPA`)))
            (:`Is Not Valid`
              (`KismetSystemLibrary.Delay` 0.1 :!label _label)))
          (set `self.IsParrySuccessful` false))
        (:`then_1`
          (bind _returnvalue_6 (`AnimInstance.Montage_Play` (`SkeletalMeshComponent.GetAnimInstance` (`Actor.GetComponentByClass` (`self.GetOwner`) "/Script/Engine.SkeletalMeshComponent")) (`/Game/ParryAttackSystem/PAS_Assets/ParryComponent/AC_ParryAttack.Reaction Montage (Defender)` (`self.AttackerPA`)) 1.0 "MontageLength" 0.0 true))
          (set `self.IsParryMontagePlaying` true)
          (`KismetSystemLibrary.Delay` (* _returnvalue_6 0.5))
          (set `self.IsParryMontagePlaying` false)))
      (else
        (goto _label)))))

(fn `CalculateCounterTransform`
  (bind _attacker (`self.Attacker`))
  (bind (_returnvalue_location _returnvalue_rotation) (`KismetMathLibrary.BreakTransform` (`Actor.GetTransform` (`self.Attacker`))))
  (bind (_returnvalue_roll _returnvalue_pitch _returnvalue_yaw) (`KismetMathLibrary.BreakRotator` (`KismetMathLibrary.Conv_VectorToRotator` (* (`KismetMathLibrary.Normal` (- (`Actor.K2_GetActorLocation` _attacker) (`Actor.K2_GetActorLocation` (`self.GetOwner`)))) -1.0))))
  (bind (_returnvalue_roll_2 _returnvalue_pitch_2 _returnvalue_yaw_2) (`KismetMathLibrary.BreakRotator` (`KismetMathLibrary.Conv_VectorToRotator` (* (`KismetMathLibrary.Normal` (- (`Actor.K2_GetActorLocation` (`self.GetOwner`)) (`Actor.K2_GetActorLocation` (`self.Attacker`)))) -1.0))))
  ;[1 1 1] Smooth interpolate positions (Attacker and victim)
  (`Actor.K2_SetActorRotation` (`self.GetOwner`) (`KismetMathLibrary.MakeRotator` 0.0 0.0 _returnvalue_yaw_2) true)
  (`Actor.K2_SetActorRotation` (`self.Attacker`) (.rotation (`KismetMathLibrary.MakeTransform` (`KismetMathLibrary.VLerp` (`Actor.K2_GetActorLocation` (`self.GetOwner`)) (+ (* (`KismetMathLibrary.Normal` (- (`Actor.K2_GetActorLocation` (`self.GetOwner`)) (`Actor.K2_GetActorLocation` _attacker))) (`self.FinisherDistance`)) (`Actor.K2_GetActorLocation` (`self.Attacker`))) 1.0) (`KismetMathLibrary.RLerp` _returnvalue_rotation (`KismetMathLibrary.MakeRotator` 0.0 0.0 _returnvalue_yaw) 1.0 true) (`Actor.GetActorScale3D` (`self.GetOwner`)))) false)
  (`Actor.K2_SetActorLocation` (`self.GetOwner`) (.location (`KismetMathLibrary.MakeTransform` (`KismetMathLibrary.VLerp` (`Actor.K2_GetActorLocation` (`self.GetOwner`)) (+ (* (`KismetMathLibrary.Normal` (- (`Actor.K2_GetActorLocation` (`self.GetOwner`)) (`Actor.K2_GetActorLocation` _attacker))) (`self.FinisherDistance`)) (`Actor.K2_GetActorLocation` (`self.Attacker`))) 1.0) (`KismetMathLibrary.RLerp` _returnvalue_rotation (`KismetMathLibrary.MakeRotator` 0.0 0.0 _returnvalue_yaw) 1.0 true) (`Actor.GetActorScale3D` (`self.GetOwner`)))) false false))

(fn `CalculateFinisherTransform`
  (bind _returnvalue (`self.GetOwner`))
  (bind _victimactor (`self.VictimActor`))
  (bind (_returnvalue_location _returnvalue_rotation) (`KismetMathLibrary.BreakTransform` (`Actor.GetTransform` (`self.VictimActor`))))
  (bind (_returnvalue_roll _returnvalue_pitch _returnvalue_yaw) (`KismetMathLibrary.BreakRotator` (`Actor.K2_GetActorRotation` _returnvalue)))
  (bind (_returnvalue_roll_2 _returnvalue_pitch_2 _returnvalue_yaw_2) (`KismetMathLibrary.BreakRotator` (`KismetMathLibrary.Conv_VectorToRotator` (* (`KismetMathLibrary.Normal` (- (`Actor.K2_GetActorLocation` _victimactor) (`Actor.K2_GetActorLocation` (`self.GetOwner`)))) -1.0))))
  (bind (_returnvalue_roll_3 _returnvalue_pitch_3 _returnvalue_yaw_3) (`KismetMathLibrary.BreakRotator` (`KismetMathLibrary.Conv_VectorToRotator` (* (`KismetMathLibrary.Normal` (- (`Actor.K2_GetActorLocation` (`self.GetOwner`)) (`Actor.K2_GetActorLocation` (`self.VictimActor`)))) -1.0))))
  ;[1 1 1] Smooth interpolate positions (Attacker and victim)
  (`Actor.K2_SetActorRotation` (`self.GetOwner`) (`KismetMathLibrary.MakeRotator` 0.0 0.0 _returnvalue_yaw_3) true)
  (`Actor.K2_SetActorRotation` (`self.VictimActor`) (.rotation (`KismetMathLibrary.MakeTransform` (`KismetMathLibrary.VLerp` (`Actor.K2_GetActorLocation` (`self.GetOwner`)) (+ (* (`KismetMathLibrary.Normal` (- (`Actor.K2_GetActorLocation` (`self.GetOwner`)) (`Actor.K2_GetActorLocation` _victimactor))) (`self.FinisherDistance`)) (`Actor.K2_GetActorLocation` (`self.VictimActor`))) 1.0) (`KismetMathLibrary.RLerp` _returnvalue_rotation (`KismetMathLibrary.MakeRotator` 0.0 0.0 (select `bool` (`self.FinishFromBehind?`) :`false` _returnvalue_yaw_2 :`true` _returnvalue_yaw :!type "Float (double-precision)")) 1.0 true) (`Actor.GetActorScale3D` _returnvalue))) false)
  (`Actor.K2_SetActorLocation` (`self.GetOwner`) (.location (`KismetMathLibrary.MakeTransform` (`KismetMathLibrary.VLerp` (`Actor.K2_GetActorLocation` (`self.GetOwner`)) (+ (* (`KismetMathLibrary.Normal` (- (`Actor.K2_GetActorLocation` (`self.GetOwner`)) (`Actor.K2_GetActorLocation` _victimactor))) (`self.FinisherDistance`)) (`Actor.K2_GetActorLocation` (`self.VictimActor`))) 1.0) (`KismetMathLibrary.RLerp` _returnvalue_rotation (`KismetMathLibrary.MakeRotator` 0.0 0.0 (select `bool` (`self.FinishFromBehind?`) :`false` _returnvalue_yaw_2 :`true` _returnvalue_yaw :!type "Float (double-precision)")) 1.0 true) (`Actor.GetActorScale3D` _returnvalue))) false false))

(fn `Check Stealth Kill`
  (returns (IsStealth :type Boolean))
  (bind _victimactor (`self.VictimActor`))
  (bind (_returnvalue_roll _returnvalue_pitch _returnvalue_yaw) (`KismetMathLibrary.BreakRotator` (`KismetMathLibrary.NormalizedDeltaRotator` (`Actor.K2_GetActorRotation` _victimactor) (`KismetMathLibrary.FindLookAtRotation` (`Actor.K2_GetActorLocation` _victimactor) (`Actor.K2_GetActorLocation` (`self.GetOwner`))))))
  (return (or (`KismetMathLibrary.InRange_FloatFloat` _returnvalue_yaw -180.0 -105.0) (`KismetMathLibrary.InRange_FloatFloat` _returnvalue_yaw 105.0 180.0))))

(fn `IsParryMontagePlaying?`
  (returns (IsParryMontagePlaying :type Boolean))
  (return (`self.IsParryMontagePlaying`)))

(fn `Parry`
  (params (Attacker :type "Actor Object Reference"))
  (returns (ParryFailed :type Boolean))
  (`self.AttackerCheck` Attacker)
  (if (and (`self.IsTryParry?`) (`/Game/ParryAttackSystem/PAS_Assets/ParryComponent/AC_ParryAttack.Can be Parried?` (`self.AttackerPA`)))
    (set `self.IsParrySuccessful` true)
    (`self.Parry Event`)
    (else
      (set `self.IsParrySuccessful` false)))
  (return (not (`self.IsParrySuccessful`))))

(fn `SetMovement/Collision`
  (params (TargetActor :type "Actor Object Reference") (NewMovementMode :type "EMovementMode Enum" :default "MOVE_None") (NewType :type "ECollisionEnabled Enum" :default "NoCollision"))
  (`CharacterMovementComponent.SetMovementMode` (`Actor.GetComponentByClass` TargetActor "/Script/Engine.CharacterMovementComponent") NewMovementMode 0)
  (`PrimitiveComponent.SetCollisionEnabled` (`Actor.GetComponentByClass` TargetActor "/Script/Engine.CapsuleComponent") NewType))

(fn `SetVictim`
  (bind _returnvalue (`self.GetOwner`))
  (bind _returnvalue_2 (`Actor.K2_GetActorLocation` _returnvalue))
  (bind _outhit (`KismetSystemLibrary.CapsuleTraceSingle` _returnvalue_2 (+ _returnvalue_2 (* (`SceneComponent.GetForwardVector` (`Actor.RootComponent` _returnvalue)) (`self.Finisher Distance Range`))) 35.0 48.0 "TraceTypeQuery2" false (`|MakeArray` (`self.GetOwner`))))
  (bind _output_get (set `self.VictimFound` (`GameplayStatics.BreakHitResult` _outhit)))
  (if _output_get
    (bind _output_get_2 (set `self.VictimActor` (`.HitActor` (`GameplayStatics.BreakHitResult` _outhit))))
    (bind _returnvalue_3 (`Actor.GetComponentByClass` _output_get_2 "AC_ParryAttack_C"))
    (`/Engine/EditorBlueprintResources/StandardMacros.IsValid` _returnvalue_3
      (:`Is Valid`
        (set `self.FinishFromBehind?` (`self.Check Stealth Kill`))
        (bind _returnvalue_4 (`|GetDataTableRow` "/Game/ParryAttackSystem/PAS_Assets/ParryComponent/DT_Finishers.DT_Finishers" (`/Game/ParryAttackSystem/PAS_Assets/ParryComponent/AC_ParryAttack.Character Name` _returnvalue_3))
          (:`then`
            (bind (_frontfinishers _backfinishers) (break `/Game/ParryAttackSystem/PAS_Assets/ParryComponent/F_Finishers` _returnvalue_4))
            (set `self.Front Finishers` _frontfinishers)
            (set `self.Back Finishers` _backfinishers)))))))