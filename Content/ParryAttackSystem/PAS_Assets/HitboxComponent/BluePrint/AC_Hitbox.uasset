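; Actor component that detects melee and ranged attack hits for its owner, fed by hitbox notify calls and routed through Srv trace events.
; Melee sweeps sphere, line or box traces from each socket's previously stored position to its current one, using body bones or weapon sockets.
; Ranged attacks use a multi-sphere trace.
; Each actor hit is broadcast once via the HitResult dispatcher until EndAttackTrace clears the stored data.
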(event `/Game/ParryAttackSystem/PAS_Assets/HitboxComponent/BluePrint/BI_Hitbox.BeginMeleeAttackTrace`
  (params (MeleeAttackType :type "/Game/ParryAttackSystem/PAS_Assets/HitboxComponent/Enums/E_Melee_Attack_Type Enum" :default "NewEnumerator0") (TraceType :type "/Game/ParryAttackSystem/PAS_Assets/HitboxComponent/Enums/E_TraceType Enum" :default "NewEnumerator0") (BoneName :type "Array of Name (by ref)") (TraceSize :type "Float (double-precision)"))
  ;[0 0 0] Collect Hitbox Info From Hitbox Notify
  (`self.Melee Hitbox Trace(Srv)` TraceType MeleeAttackType TraceSize BoneName))

(event `/Game/ParryAttackSystem/PAS_Assets/HitboxComponent/BluePrint/BI_Hitbox.BeginRangedAttackTrace`
  (params (TraceHeight :type "Float (double-precision)") (TraceRadius :type "Float (double-precision)") (TraceForwardLength :type "Float (double-precision)"))
  ;[0 0 0] Collect Hitbox Info From Hitbox Notify
  (`self.Ranged Hitbox Trace(Srv)` TraceHeight TraceRadius TraceForwardLength))

(event `HitResultEvent`
  (params (HitResult :type "HitResult Structure"))
  ;[0 0.01223 0.07187] Hit Result Dispatcher
  (`self.HitResult` HitResult))

(event `/Game/ParryAttackSystem/PAS_Assets/HitboxComponent/BluePrint/BI_Hitbox.InitWeapon`
  (params (WeaponMesh :type "PrimitiveComponent Object Reference"))
  ;[0.003389 0.03438 0] Initiate Player & Weapon
  (set `self.Weapon Mesh` WeaponMesh))

(event `/Game/ParryAttackSystem/PAS_Assets/HitboxComponent/BluePrint/BI_Hitbox.EndAttackTrace`
  ;[0.04271 0 0.009448] Clear Stored info
  (`KismetArrayLibrary.Array_Clear` (`self.Trace Start`))
  (`KismetArrayLibrary.Array_Clear` (`self.Hit Actor`)))

(event `Ranged Hitbox Trace(Srv)`
  (params (TraceHeight :type "Float (double-precision)") (TraceRadius :type "Float (double-precision)") (TraceForwardLength :type "Float (double-precision)"))
  (bind (_returnvalue _returnvalue2) (`self.RangedTraceLocation`))
  ;[0 0 0] Start Ranged Hitbox Trace
  (set `self.Trace Height` TraceHeight)
  (set `self.TraceSize` TraceRadius)
  (set `self.TraceDistance` TraceForwardLength)
  (bind _outhits (`KismetSystemLibrary.SphereTraceMulti` _returnvalue _returnvalue2 (`self.TraceSize`) (`self.Trace Channel`) false (`|MakeArray` (`self.GetOwner`)) (`self.Draw Debug Type`) true (`self.Trace Color`) (`self.Trace Hit Color`) (`self.Draw Time`)))
  (for _array_element _outhits
    (bind (_bblockinghit _binitialoverlap _time _distance _location _impactpoint _normal _impactnormal _physmat _hitactor) (`GameplayStatics.BreakHitResult` _array_element))
    (if (not (`KismetArrayLibrary.Array_Contains` (`self.Hit Actor`) _hitactor))
      (`KismetArrayLibrary.Array_AddUnique` (`self.Hit Actor`) _hitactor)
      (`self.HitResultEvent` _array_element))))

(event `Melee Hitbox Trace(Srv)`
  (params (TraceType :type "/Game/ParryAttackSystem/PAS_Assets/HitboxComponent/Enums/E_TraceType Enum" :default "NewEnumerator0") (MeleeAttackType :type "/Game/ParryAttackSystem/PAS_Assets/HitboxComponent/Enums/E_Melee_Attack_Type Enum" :default "NewEnumerator0") (TraceSize :type "Float (double-precision)") (BoneName :type "Array of Name"))
  (bind _returnvalue (`self.SelectMesh` MeleeAttackType))
  (bind _tracesize (`self.TraceSize`))
  (bind _returnvalue_2 (select `/Game/ParryAttackSystem/PAS_Assets/HitboxComponent/Enums/E_Melee_Attack_Type` MeleeAttackType :`NewEnumerator0` BoneName :`NewEnumerator1` (`SceneComponent.GetAllSocketNames` (`self.Weapon Mesh`))))
  ;[0 0 0] Based On Melee Attack Type - Start Hitbox Trace
  (set `self.TraceSize` TraceSize)
  (switch `/Game/ParryAttackSystem/PAS_Assets/HitboxComponent/Enums/E_TraceType` TraceType
    (:`NewEnumerator0`
      (for (_array_element _array_index) _returnvalue_2
        (bind _output_get (set `self.Trace End` (`SceneComponent.GetSocketLocation` (`self.SelectMesh` MeleeAttackType) _array_element)))
        (`|ExecutionSequence`
          (:`then_0`
            (bind _output (`|GetArrayItem` (`self.Trace Start`) _array_index))
            (if (!= _output (0.0 0.0 0.0))
              (bind _outhits (`KismetSystemLibrary.SphereTraceMulti` _output (`self.Trace End`) (`self.TraceSize`) (`self.Trace Channel`) false (`|MakeArray` (`self.GetOwner`)) (`self.Draw Debug Type`) true (`self.Trace Color`) (`self.Trace Hit Color`) (`self.Draw Time`)))
              (for _array_element_2 _outhits
                (bind (_bblockinghit _binitialoverlap _time _distance _location _impactpoint _normal _impactnormal _physmat _hitactor) (`GameplayStatics.BreakHitResult` _array_element_2))
                (if (not (`KismetArrayLibrary.Array_Contains` (`self.Hit Actor`) _hitactor))
                  (`KismetArrayLibrary.Array_AddUnique` (`self.Hit Actor`) _hitactor)
                  (`self.HitResultEvent` _array_element_2)))))
          (:`then_1`
            (`KismetArrayLibrary.Array_Set` (`self.Trace Start`) _array_index (+ _output_get (0.0 0.0 1.0)) true)))))
    (:`NewEnumerator1`
      (for (_array_element_3 _array_index_2) _returnvalue_2
        (bind _output_get_2 (set `self.Trace End` (`SceneComponent.GetSocketLocation` (`self.SelectMesh` MeleeAttackType) _array_element_3)))
        (`|ExecutionSequence`
          (:`then_0`
            (bind _output_2 (`|GetArrayItem` (`self.Trace Start`) _array_index_2))
            (if (!= _output_2 (0.0 0.0 0.0))
              (bind _outhits_2 (`KismetSystemLibrary.LineTraceMulti` _output_2 (`self.Trace End`) (`self.Trace Channel`) false (`|MakeArray` (`self.GetOwner`)) (`self.Draw Debug Type`) true (`self.Trace Color`) (`self.Trace Hit Color`) (`self.Draw Time`)))
              (for _array_element_4 _outhits_2
                (bind (_bblockinghit_2 _binitialoverlap_2 _time_2 _distance_2 _location_2 _impactpoint_2 _normal_2 _impactnormal_2 _physmat_2 _hitactor_2) (`GameplayStatics.BreakHitResult` _array_element_4))
                (if (not (`KismetArrayLibrary.Array_Contains` (`self.Hit Actor`) _hitactor_2))
                  (`KismetArrayLibrary.Array_AddUnique` (`self.Hit Actor`) _hitactor_2)
                  (`self.HitResultEvent` _array_element_4)))))
          (:`then_1`
            (`KismetArrayLibrary.Array_Set` (`self.Trace Start`) _array_index_2 (+ _output_get_2 (0.0 0.0 1.0)) true)))))
    (:`NewEnumerator2`
      (for (_array_element_5 _array_index_3) _returnvalue_2
        (bind _output_get_3 (set `self.Trace End` (`SceneComponent.GetSocketLocation` _returnvalue _array_element_5)))
        (`|ExecutionSequence`
          (:`then_0`
            (bind _output_3 (`|GetArrayItem` (`self.Trace Start`) _array_index_3))
            (if (!= _output_3 (0.0 0.0 0.0))
              (bind _outhits_3 (`KismetSystemLibrary.BoxTraceMulti` _output_3 (`self.Trace End`) (`KismetMathLibrary.MakeVector` _tracesize _tracesize _tracesize) (`SceneComponent.GetSocketRotation` _returnvalue _array_element_5) (`self.Trace Channel`) false (`|MakeArray` (`self.GetOwner`)) (`self.Draw Debug Type`) true (`self.Trace Color`) (`self.Trace Hit Color`) (`self.Draw Time`)))
              (for _array_element_6 _outhits_3
                (bind (_bblockinghit_3 _binitialoverlap_3 _time_3 _distance_3 _location_3 _impactpoint_3 _normal_3 _impactnormal_3 _physmat_3 _hitactor_3) (`GameplayStatics.BreakHitResult` _array_element_6))
                (if (not (`KismetArrayLibrary.Array_Contains` (`self.Hit Actor`) _hitactor_3))
                  (`KismetArrayLibrary.Array_AddUnique` (`self.Hit Actor`) _hitactor_3)
                  (`self.HitResultEvent` _array_element_6)))))
          (:`then_1`
            (`KismetArrayLibrary.Array_Set` (`self.Trace Start`) _array_index_3 (+ _output_get_3 (0.0 0.0 1.0)) true)))))))